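; Blueprint function library of easing curves that remap an input value for interpolation.
; It provides quadratic ease-in and ease-out, bounce ease-in and ease-out, and an elastic ease-in as separate functions.
; The bounce variants multiply an exponential envelope by the absolute value of a sine or cosine wave.
; The elastic variant scales a sine wave by the fourth power of the input.
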(fn EaseinQuad
  (params (Val :type Float%20%28double-precision%29))
  (return (* Val Val)))

(fn EaseOutBounce
  (params (Val :type Float%20%28double-precision%29))
  (return (- 1.0 (* (Math|Float|Power 2.0 (* Val -6.0)) (Math|Float|Absolute(Float) (Math|Trig|Cos(Radians) (* Val (Math|Trig|GetPI) 3.5)))))))

(fn EaseOutQuad
  (params (Val :type Float%20%28double-precision%29))
  (return (- 1.0 (* (- 1.0 Val) (- 1.0 Val)))))

(fn EaseinBounce
  (params (Val :type Float%20%28double-precision%29))
  (return (* (Math|Float|Power 2.0 (* (- Val 1.0) 6.0)) (Math|Float|Absolute(Float) (Math|Trig|Sin(Radians) (* Val (Math|Trig|GetPI) 3.5))))))

(fn EaseinElastic
  (params (Val :type Float%20%28double-precision%29))
  (bind _returnvalue (* Val Val))
  (return (* _returnvalue _returnvalue (Math|Trig|Sin(Radians) (* Val (Math|Trig|GetPI) 4.5)))))